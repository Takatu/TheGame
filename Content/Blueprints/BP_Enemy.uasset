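; Enemy actor that travels along a referenced spline, driven on Tick by a two-state machine: Spawn and Attack.
; Spawn shrinks an offset along the actor's up vector at a tenth of its speed, switching to Attack when it reaches zero.
; Both states share one movement step that sets location and rotation from the spline, then advances the distance by speed and delta time.
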(event `self.ReceiveTick`
  (params (DeltaSeconds :type "Float (single-precision)"))
  (bind _offset (`self.Offset`))
  (bind _splinepos (`self.SplinePos`))
  (bind _spline1 (`/Game/Blueprints/BP_Spline.Spline1` (`self.Spline`)))
  (switch `/Game/Blueprints/E_EnemyState` (`self.State`)
    (:`NewEnumerator0`
      (set `self.Offset` (- _offset (* (* (`self.Speed`) 0.1) DeltaSeconds)))
      (if (<= _offset 0.0)
        (set `self.Offset` 0.0)
        (set `self.State` "NewEnumerator1")))
    (:`NewEnumerator1`
      _))
  (`self.SetActorLocationAndRotation` (+ (`SplineComponent.GetWorldLocationAtDistanceAlongSpline` _spline1 _splinepos) (* (`self.GetActorUpVector`) (`self.Offset`))) (`SplineComponent.GetWorldRotationAtDistanceAlongSpline` _spline1 _splinepos))
  (set `self.SplinePos` (+ (`self.SplinePos`) (* DeltaSeconds (`self.Speed`)))))

(fn `UserConstructionScript`)