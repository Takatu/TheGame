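; BP_GravityVolume is a temporary volume actor that pushes whatever components overlap its Trigger in a set direction.
; Every Tick it applies ForceDirection times Force to each overlapping component, scaled by that component's mass so the acceleration is mass-independent, like gravity.
; On BeginPlay it sets its life span from LifeTime, so the volume destroys itself when that time runs out.
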(event `self.ReceiveTick`
  (params (DeltaSeconds :type "Float (single-precision)"))
  ;[1 1 1] Apply force to every component in the Volume
  (for _array_element (`PrimitiveComponent.GetOverlappingComponents` (`self.Trigger`))
    (`PrimitiveComponent.AddForce` _array_element (* (* (`self.Force Direction`) (`self.Force`)) (`PrimitiveComponent.GetMass` _array_element)) "None")))

(event `self.ReceiveBeginPlay`
  ;[1 1 1] Set the Life Span
  (`self.SetLifeSpan` (`self.Life Time`)))

(fn `UserConstructionScript`)