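; BP_Ghost is a ghost that chases one player and dodges another, the Scarer, when that player faces it.
; On server Tick, sphere overlaps within SightRadius fill Target from the first player found, then Scarer from the second; movement needs both.
; A dot product check on the Scarer's facing switches between swept movement toward Target and unswept movement out of the Scarer's line of view.
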(event `self.ReceiveTick`
  (params (DeltaSeconds :type "Float (single-precision)"))
  (bind _returnvalue (`self.K2_GetActorLocation`))
  (bind _returnvalue_2 (`self.K2_GetActorLocation`))
  (bind _target (`self.Target`))
  (bind _scarer (`self.Scarer`))
  (bind _playerclass (`self.PlayerClass`))
  (`/Engine/EditorBlueprintResources/ActorMacros.Switch Has Authority`
    (:`Authority`
      (`/Engine/EditorBlueprintResources/StandardMacros.IsValid` _target
        (:`Is Valid`
          (`/Engine/EditorBlueprintResources/StandardMacros.IsValid` _scarer
            (:`Is Valid`
              (bind _returnvalue_3 (`self.GetDotProductTo` _scarer self))
              (if (>= _returnvalue_3 0.9)
                ;[1 1 1] Avoid Scarer
                (`self.K2_SetActorLocation` (+ (* (`KismetMathLibrary.Normal` (- (`KismetMathLibrary.Normal` (- _returnvalue (`self.K2_GetActorLocation` (`self.Scarer`)))) (`KismetMathLibrary.Normal` (`self.GetActorForwardVector` (`self.Scarer`))))) (* DeltaSeconds (`self.Speed`))) _returnvalue))
                (else
                  ;[1 1 1] Follow Target
                  (`self.K2_SetActorLocation` (+ _returnvalue_2 (* (`KismetMathLibrary.Normal` (- (`self.K2_GetActorLocation` _target) _returnvalue_2)) (* (`self.Speed`) DeltaSeconds))) true))))
            (:`Is Not Valid`
              ;[1 1 1] Find Scarer
              (bind (_outactors _returnvalue_4) (`KismetSystemLibrary.SphereOverlapActors_NEW` (`self.K2_GetActorLocation`) (`self.Sight Radius`) (`|MakeArray` "ObjectTypeQuery3" :!type "EngineTypes.EObjectTypeQuery Enum") _playerclass))
              (if _returnvalue_4
                (set `self.Scarer` (`KismetArrayLibrary.Array_Get` _outactors 1))))))
        (:`Is Not Valid`
          ;[1 1 1] Find Target
          (bind (_outactors_2 _returnvalue_5) (`KismetSystemLibrary.SphereOverlapActors_NEW` (`self.K2_GetActorLocation`) (`self.Sight Radius`) (`|MakeArray` "ObjectTypeQuery3" :!type "EngineTypes.EObjectTypeQuery Enum") _playerclass))
          (if _returnvalue_5
            (set `self.Target` (`KismetArrayLibrary.Array_Get` _outactors_2))))))))

(fn `UserConstructionScript`)