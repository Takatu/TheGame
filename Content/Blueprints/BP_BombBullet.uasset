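; BP_BombBullet is a bomb projectile that explodes when it is hit by a CounterBullet or one of its subclasses.
; The Hit event acts only on the server, triggering the explosion, applying radial damage around the bomb and scheduling destruction after a short lifespan.
; BombExplode handles the visible result, spawning an enlarged explosion emitter, then disabling collision and hiding the actor.
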(event `self.ReceiveHit`
  (params (MyComp :type "PrimitiveComponent Object Reference") (Other :type "Actor Object Reference") (OtherComp :type "PrimitiveComponent Object Reference") (bSelfMoved :type Boolean) (HitLocation :type "Object.Vector Structure") (HitNormal :type "Object.Vector Structure") (NormalImpulse :type "Object.Vector Structure") (Hit :type "EngineTypes.HitResult Structure (by ref)"))
  (`/Engine/EditorBlueprintResources/ActorMacros.Switch Has Authority`
    (:`Authority`
      (if (`KismetMathLibrary.ClassIsChildOf` (`GameplayStatics.GetObjectClass` Other) (`self.Counter Bullet`))
        (`self.Bomb Explode`)
        (`GameplayStatics.ApplyRadialDamage` 25.0 (`self.K2_GetActorLocation`) 600.0)
        (`self.SetLifeSpan` 1.0)))))

(event `Bomb Explode`
  (bind _returnvalue (`GameplayStatics.SpawnEmitterAtLocation` (`self.Explosion Emitter`) (`self.K2_GetActorLocation`)))
  (`SceneComponent.SetRelativeScale3D` _returnvalue (4.0 4.0 4.0))
  (`self.SetActorEnableCollision` false)
  (`self.SetActorHiddenInGame` true))

(fn `UserConstructionScript`)