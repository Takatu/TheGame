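; BP_LeoTutorial is an experimental Blueprint that procedurally builds a curved stack of copies of one static mesh.
; Its construction script spawns mesh components in a loop driven by NumElements, parenting each to the previous one, starting from Scene1.
; Each piece is offset using its local bounds and sines of Angle, then rolled by Angle, so the bend accumulates along the chain.
; Leftover randomisation nodes are unconnected.
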(fn ConstructionScript
  (LocalVariables|SetParent%20Component (Variables|Default|GetScene1))
  (for _index (range 0 (Variables|Default|GetNum%20Elements))
    (bind _returnvalue (AddComponent|AddStaticMeshComponent false))
    (Components|StaticMesh|SetStaticMesh _returnvalue (Variables|Default|GetStatic%20Mesh))
    (Class|SceneComponent|Attachto _returnvalue (LocalVariables|GetParent%20Component) "None" "KeepRelativeOffset")
    (LocalVariables|SetRandom%20Rotation (Class|KismetMathLibrary|MakeRot 0.0 0.0 (Variables|Default|GetAngle)))
    (Transformation|SetRelativeLocation _returnvalue (* (Math|Vector|MakeVector 0.0 (* (Math|Trig|Sin(Degrees) (/ (.Roll (Class|KismetMathLibrary|BreakRot (LocalVariables|GetRandom%20Rotation))) 2.0)) (- (.Y (Math|Vector|BreakVector (.Max (Components|StaticMesh|GetLocalBounds _returnvalue)))) (.Y (Math|Vector|BreakVector (.Min (Components|StaticMesh|GetLocalBounds _returnvalue)))))) (- (- (.Z (Math|Vector|BreakVector (.Max (Components|StaticMesh|GetLocalBounds _returnvalue)))) (.Z (Math|Vector|BreakVector (.Min (Components|StaticMesh|GetLocalBounds _returnvalue))))) (Math|Trig|Sin(Degrees) (.Roll (Class|KismetMathLibrary|BreakRot (LocalVariables|GetRandom%20Rotation)))))) 1.0) false)
    (Transformation|SetRelativeRotation _returnvalue (LocalVariables|GetRandom%20Rotation) false)
    (LocalVariables|SetParent%20Component _returnvalue)))