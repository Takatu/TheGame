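; A door Blueprint that swings open once enough toggle inputs are active and closes when they drop below that count.
; Toggle runs only on authority, counting on/off signals against ToggleCount, with StatePersistant intended to latch the state.
; A DoorOpen timeline drives the door's yaw forward or in reverse.
; Collision turns off once fully open and returns once fully closed.
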(event `self.Toggle`
  (params (`On/off` :type Boolean))
  (bind _returnvalue (>= (`self.ToggleCounter`) (`self.Toggle Count`)))
  (`/Engine/EditorBlueprintResources/ActorMacros.Switch Has Authority`
    (:`Authority`
      (if (`self.StatePersistant`)
        (if (not (`self.On/off`))
          (if `On/off` :!label _label
            (set `self.ToggleCounter` (+ (`self.ToggleCounter`) 1))
            (else
              (set `self.ToggleCounter` (- (`self.ToggleCounter`) 1))))
          (if (!= (`self.On/off`) _returnvalue)
            (set `self.On/off` _returnvalue)
            (if (`self.On/off`)
              (`self.OpenDoor`)
              (else
                (`self.CloseDoor`)))))
        (else
          (goto _label))))))

(event `OpenDoor`
  (bind _door (`self.Door`))
  (bind (_direction _dooryaw) (`Timeline|DoorOpen` :!label _label_2)
    (:`Update`
      (`SceneComponent.SetRelativeRotation` _door (`KismetMathLibrary.MakeRot` 0.0 _dooryaw) false))
    (:`Finished`
      (switch `TimelineComponent.ETimelineDirection` _direction
        (:`Forward`
          (`PrimitiveComponent.SetCollisionEnabled` _door "NoCollision"))
        (:`Backward`
          (`PrimitiveComponent.SetCollisionEnabled` _door "QueryAndPhysics"))))))

(event `CloseDoor`
  (goto _label_2 :!via `Reverse`))

(fn `UserConstructionScript`)