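; BP_HiddenOnClient is an actor whose static mesh is hidden on clients and visible on the authority until damage reveals it.
; BeginPlay uses an authority switch to set that initial visibility, and the construction script stores a dynamic material instance of the mesh.
; On damage, ObjectDiscovered shows the mesh and applies the basic wall material, then the actor's lifespan is set to LifetimeAfterHit.
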(event `self.ReceiveBeginPlay`
  (bind _staticmesh (`self.StaticMesh`))
  (`/Engine/EditorBlueprintResources/ActorMacros.Switch Has Authority`
    (:`Authority`
      (`SceneComponent.SetVisibility` _staticmesh true false))
    (:`Remote`
      (`SceneComponent.SetVisibility` _staticmesh false false))))

(event `self.ReceiveAnyDamage`
  (params (Damage :type "Float (single-precision)") (DamageType :type "DamageType Object Reference") (InstigatedBy :type "Controller Object Reference") (DamageCauser :type "Actor Object Reference"))
  (`self.Object Discovered`)
  (`self.SetLifeSpan` (`self.lifetime after hit`)))

(event `Object Discovered`
  (bind _staticmesh (`self.StaticMesh`))
  (`SceneComponent.SetVisibility` _staticmesh true false)
  (`PrimitiveComponent.SetMaterial` _staticmesh 0 "/Game/Materials/M_Basic_Wall.M_Basic_Wall"))

(fn `UserConstructionScript`
  (bind _returnvalue (`PrimitiveComponent.CreateDynamicMaterialInstance` (`self.StaticMesh`) 0 null))
  (set `self.Material` _returnvalue))